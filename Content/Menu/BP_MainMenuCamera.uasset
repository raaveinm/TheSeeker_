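; Main menu camera actor that shows the menu overlay widget and can be locked for the length of a sequence.
; BeginPlay creates the overlay and adds it to the viewport, while the construction script enables the camera-follow flag.
; LockCamera sets that flag, then either re-adds the overlay or removes it and eases the camera component to its default move target over the given duration.
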(event EventBeginPlay
  (bind _returnvalue (UserInterface|CreateWidget "/Game/Menu/Widgets/WG_MenuOverlay.WG_MenuOverlay_C"))
  (bind _output_get (Variables|Default|SetMenu%20Widget _returnvalue))
  (UserInterface|Viewport|AddtoViewport _output_get 0))

(event EventLockCamera
  (params (Can%20Camera%20Move :type Boolean) (Sequence%20Lenght :type Float%20%28double-precision%29))
  (bind _output_get (Variables|Default|SetCameraFollowEnabled Can%20Camera%20Move))
  (if _output_get
    (UserInterface|Viewport|AddtoViewport (Variables|Default|GetMenu%20Widget) 0)
    (else
      (Components|MoveComponentTo (Variables|Default|GetCameraComp) "0, 0, 0" "0, 0, 0" true false Sequence%20Lenght false)
      (Widget|RemovefromParent (Variables|Default|GetMenu%20Widget)))))

(fn ConstructionScript
  (Variables|Default|SetCameraFollowEnabled true))