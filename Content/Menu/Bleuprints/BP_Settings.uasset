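; Main menu Settings cube that, when clicked, plays the LookOnSettings level sequence and opens the settings widget.
; The sequence player is created once and reused, playing forward to enter and in reverse when settings exit.
; A FlipFlop on the end of the cutscene alternates between showing WG_Settings and restoring the centered menu cursor.
; HideShowMouse toggles cursor, click events and input mode, messaging the pawn to lock its camera with the sequence length.
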(event Custom|Exit%20Options
  (bind _returnvalue (Game|GetPlayerController 0))
  ;[0.15 0.15 0.15 0.5] Cutsceen's Logic
  ;;[0.15 0.15 0.15 0.5] Close Settings
  (Variables|/Script/Engine.PlayerController|SetbShowMouseCursor _returnvalue false)
  (Input|SetInputModeGameOnly _returnvalue false)
  (Class|MovieSceneSequencePlayer|PlayReverse (Variables|Default|GetOptions%20Animation)))

(event Custom|End%20Of%20Cutsceen
  (bind _returnvalue (Game|GetPlayerController 0))
  (bind (_sizex _sizey) (HUD|GetViewportSize _returnvalue))
  ;[0.15 0.15 0.15 0.5] Cutsceen's Logic
  (Utilities|FlowControl|FlipFlop
    (:A
      ;;[0.15 0.15 0.15 0.5] Open Settings
      (bind _returnvalue_2 (UserInterface|CreateWidget "/Game/Menu/Widgets/WG_Settings.WG_Settings_C"))
      (EventDispatchers|BindEventtoOnExit _returnvalue_2 (EventDispatchers|CreateEvent :!event Custom|Exit%20Options))
      (UserInterface|Viewport|AddtoViewport _returnvalue_2 0))
    (:B
      ;;[0.15 0.15 0.15 0.5] Get Back to Main Menu
      (Class|PlayerController|SetMouseLocation _returnvalue (/ _sizex 2) (/ _sizey 2))
      (CallFunction|Hide/ShowMouse true))))

(event EventPerformAction
  ;[0.15 0.15 0.15 0.5] Click on Settings Cube
  (|CallParentFunction)
  (Variables|Default|GetOptions%20Animation
    (:then
      _)
    (:else
      (bind _returnvalue (Sequencer|Player|CreateLevelSequencePlayer "/Game/Menu/Sequences/LookOnSettings.LookOnSettings" (Variables|Default|GetSequence%20Settings)))
      (bind _output_get (Variables|Default|SetOptions%20Animation _returnvalue))
      (EventDispatchers|BindEventtoOnFinished _output_get (EventDispatchers|CreateEvent :!event Custom|End%20Of%20Cutsceen))))
  (Sequencer|Player|Play (Variables|Default|GetOptions%20Animation) :!class /Script/MovieScene.MovieSceneSequencePlayer)
  (CallFunction|Hide/ShowMouse false))

(fn ConstructionScript
  (|CallParentFunction))

(fn Hide/ShowMouse
  (params (Show%20Mouse%20Cursor :type Boolean))
  (bind _returnvalue (Game|GetPlayerController 0))
  (bind _options_animation (Variables|Default|GetOptions%20Animation))
  (bind _returnvalue_2 (Class|MovieSceneSequencePlayer|GetEndTime _options_animation))
  (bind _output_get (Variables|/Script/Engine.PlayerController|SetbShowMouseCursor _returnvalue Show%20Mouse%20Cursor))
  (bind _output_get_2 (Variables|/Script/Engine.PlayerController|SetbEnableMouseOverEvents _returnvalue _output_get))
  (bind _output_get_3 (Variables|/Script/Engine.PlayerController|SetbEnableClickEvents _returnvalue _output_get_2))
  (Class|BPIMainMenu|LockCamera(Message) (Game|Player|GetPlayerPawn 0) _output_get_3 (/ (.value (.frame _returnvalue_2)) (.numerator (.framerate _returnvalue_2))))
  (if _output_get_3
    (Input|SetInputModeGameandUI _returnvalue 0 "DoNotLock" true false)
    (else
      (Input|SetInputModeGameOnly _returnvalue false))))