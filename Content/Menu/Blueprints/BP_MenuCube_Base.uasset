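; BP_MenuCube_Base is a base Blueprint for cube buttons in the game's menu, with hover, exit and press feedback.
; Its hover and press events play their own sounds on the Audio component, and hover lights a glow that exit or press clears.
; SetHoverGlow drives the glow through a vector parameter on the mesh materials.
; The construction script sets the text label from the class display name, so subclasses label themselves.
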(event EventPerformAction
  (bind _audio (Variables|Default|GetAudio))
  (Audio|Components|Audio|SetSound _audio "/Game/Menu/Sound/SFX_SpaceButtonPressed.SFX_SpaceButtonPressed")
  (Audio|Components|Audio|Play _audio 0.0)
  (CallFunction|SetHoverGlow "0, 0, 0"))

(event EventOnHoverEnter
  (bind _audio (Variables|Default|GetAudio))
  (Audio|Components|Audio|SetSound _audio "/Game/Menu/Sound/SFX_SpaceButtonHovered.SFX_SpaceButtonHovered")
  (Audio|Components|Audio|Play _audio 0.0)
  (CallFunction|SetHoverGlow "50.000000,50.000000,50.000000"))

(event EventOnHoverExit
  (CallFunction|SetHoverGlow "0, 0, 0"))

(fn ConstructionScript
  (Rendering|Components|TextRender|SetText (Variables|Default|GetTextRender) (Utilities|Text|ToText(String) (Utilities|GetClassDisplayName (Utilities|GetClass self)))))

(fn SetHoverGlow
  (params (ParameterValue :type Vector))
  (bind _output_get (Variables|Default|SetDisplacementVector ParameterValue))
  (Rendering|Material|SetVectorParameterValueonMaterials (Variables|Default|GetMeshComp) (Variables|Default|GetGlowParameter) _output_get))