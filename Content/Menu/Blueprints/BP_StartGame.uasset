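; BP_StartGame is a menu action that starts the game by opening the LVL_Ship level behind a screen fade.
; PerformAction calls the parent action, adds a WG_Fade widget to the viewport and binds to the end of its FadeOut animation, without playing it here.
; When that animation finishes, MainEvent unbinds, opens the level by name and removes the widget after a very short delay.
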(event Custom|Main%20Event
  (Class|UserWidget|UnbindfromAnimationFinished (Variables|Widgets|GetFade%20Screen) (Variables|/Game/Menu/Widgets/WG_Fade.WG_Fade_C|GetFadeOut (Variables|Widgets|GetFade%20Screen)) (delegate Custom|Main%20Event))
  (Game|OpenLevel(byName) "LVL_Ship")
  (Utilities|FlowControl|Delay 0.01)
  (Widget|RemovefromParent (Variables|Widgets|GetFade%20Screen)))

(event EventPerformAction
  (|CallParentFunction)
  (bind _returnvalue (UserInterface|CreateWidget "/Game/Menu/Widgets/WG_Fade.WG_Fade_C"))
  (bind _output_get (Variables|Widgets|SetFade%20Screen _returnvalue))
  (UserInterface|Viewport|AddtoViewport _output_get 0)
  (Class|UserWidget|BindtoAnimationFinished (Variables|Widgets|GetFade%20Screen) (Variables|/Game/Menu/Widgets/WG_Fade.WG_Fade_C|GetFadeOut _returnvalue) (delegate Custom|Main%20Event)))

(fn ConstructionScript
  (|CallParentFunction))