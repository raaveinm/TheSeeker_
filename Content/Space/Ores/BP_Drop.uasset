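; BP_Drop is a dropped ore item that pops out on spawn as a physics sphere.
; BeginPlay gives the sphere a randomized sideways and fixed upward impulse.
; ItemDrop stores the passed item data and looks up its row in DT_Ores to apply that ore's material.
; On hit, a short downward line trace checks for ground beneath the sphere and switches off physics simulation so the drop settles.
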(event OnComponentHit(Sphere)
  (params (HitComponent :type Primitive%20Component%20Object%20Reference) (OtherActor :type Actor%20Object%20Reference) (OtherComp :type Primitive%20Component%20Object%20Reference) (NormalImpulse :type Vector :default "0, 0, 0") (Hit :type Hit%20Result%20Structure%20%28by%20ref%29))
  (bind _sphere (Variables|Default|GetSphere))
  (bind _returnvalue (Transformation|GetWorldLocation _sphere))
  (bind _returnvalue_2 (Collision|LineTraceByChannel _returnvalue (+ _returnvalue "0.000000,0.000000,-50.000000") "TraceTypeQuery1" false 0 "None" true "(R=1.000000,G=0.000000,B=0.000000,A=1.000000)" "(R=0.000000,G=1.000000,B=0.000000,A=1.000000)" 1.0))
  (if _returnvalue_2
    (Physics|SetSimulatePhysics (Variables|Default|GetSphere) false)))

(event Custom|ItemDrop
  (params (ItemData :type BP%20Item%20Component%20Object%20Reference))
  (bind _output_get (Variables|Default|SetBP_ItemComponent ItemData))
  (bind _returnvalue (Utilities|GetDataTableRow "/Game/Space/Ores/DT_Ores.DT_Ores" (Variables|/Game/Space/Player/Inventory/BP_ItemComponent.BP_ItemComponent_C|GetItemRow _output_get))
    (:then
      (Rendering|Material|SetMaterial (Variables|Default|GetSphere) 0 (.orematerial _returnvalue)))))

(event EventBeginPlay
  (Physics|AddImpulse (Variables|Default|GetSphere) (Math|Vector|MakeVector (Math|Random|RandomFloatinRange -2e+01 2e+01) (Math|Random|RandomFloatinRange -2e+01 2e+01) 2e+01) "None" false))

(fn ConstructionScript)