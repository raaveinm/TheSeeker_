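; Mineable meteor ore node that configures its name, material, light color, health and loot item from a DT_Ores row.
; Max HP is the per-unit HP times a random unit count, and accumulated damage reaching one unit spawns a BP_Drop, then resets.
; Damage updates total and per-unit widget bars, which Look and EndLook show and hide.
; Destruction at zero HP tags the parent spawn point "Free".
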(event Custom|Spawn%20Loot
  (bind _returnvalue (Game|SpawnActorfromClass "/Game/Space/Ores/BP_Drop.BP_Drop_C" (Transformation|GetActorTransform) "AlwaysSpawn" "MultiplyWithRoot" 0 0))
  (Default|ItemDrop _returnvalue (Math|Random|RandomIntegerinRange 2 5) (Variables|Default|GetItem)))

(event EventLook
  (Widget|SetVisibility (Variables|/Game/Space/Ores/Widgets/WG_Meteor.WG_Meteor_C|GetWG_HpProgress (Variables|Default|GetMeteor%20Widget)) "Visible"))

(event EventEndLook
  (Widget|SetVisibility (Variables|/Game/Space/Ores/Widgets/WG_Meteor.WG_Meteor_C|GetWG_HpProgress (Variables|Default|GetMeteor%20Widget)) "Hidden"))

(event EventDamage
  (params (Damage :type Integer))
  (Variables|HP|SetDamageTaken (+ Damage (Variables|HP|GetDamageTaken)))
  (Variables|HP|SetHp (Math|Integer|Clamp(Integer) (- (Variables|HP|GetHp) Damage) 0 (Variables|HP|GetMaxHp)))
  (CallFunction|UpdateWidget)
  (if (>= (Variables|HP|GetDamageTaken) (Variables|HP|GetHPPer%20Unit))
    (CallFunction|SpawnLoot)
    (Variables|HP|SetDamageTaken 0))
  (if (<= (Variables|HP|GetHp) 0)
    (Actor|DestroyActor)))

(event EventDestroyed
  (Utilities|Array|AddUnique (Variables|/Script/Engine.Actor|GetTags (Variables|Default|GetParent%20Spawn%20Point)) "Free"))

(event EventBeginPlay
  (bind _returnvalue (Utilities|GetDataTableRow "/Game/Space/Ores/DT_Ores.DT_Ores" (Variables|Default|GetItem%20Row))
    (:then
      (CallFunction|SetVariables (.orename _returnvalue) (.orematerial _returnvalue) (.orelightcolor _returnvalue) (.hpperunit _returnvalue) (.maxquantity _returnvalue) (.item _returnvalue)))))

(fn ConstructionScript)

(fn SetVariables
  (params (OreName :type Name) (Material :type Material%20Object%20Reference) (Light%20Color :type Linear%20Color%20Structure) (Hp%20Per%20Unit :type Integer) (Max%20Quantity :type Integer) (Item :type Data%20Table%20Row%20Handle%20Structure))
  (Utilities|FlowControl|Sequence
    (:then_0
      (CallFunction|SetWidget OreName Light%20Color))
    (:then_1
      (Rendering|Material|SetMaterial (Variables|Default|GetSphere) 0 Material))
    (:then_2
      (Rendering|Components|Light|SetLightColor (Variables|Default|GetPointLight) Light%20Color true))
    (:then_3
      (Variables|HP|SetHPPer%20Unit Hp%20Per%20Unit)
      (Variables|Default|SetItem Item))
    (:then_4
      (bind _output_get (Variables|HP|SetMaxHp (* (Variables|HP|GetHPPer%20Unit) (Math|Random|RandomIntegerinRange 1 Max%20Quantity))))
      (Variables|HP|SetHp _output_get))))

(fn SetWidget
  (params (InName :type Name) (Color :type Linear%20Color%20Structure))
  (bind _aswg_meteor (Utilities|Casting|CastToWG_Meteor (UserInterface|GetWidget (Variables|Default|GetWidget))))
  (bind _output_get (Variables|Default|SetMeteor%20Widget _aswg_meteor))
  (Utilities|FlowControl|Sequence
    (:then_0
      (Rendering|Components|TextRender|SetText (Variables|/Game/Space/Ores/Widgets/WG_OreName.WG_OreName_C|GetTextBlock (Variables|/Game/Space/Ores/Widgets/WG_Meteor.WG_Meteor_C|GetWG_OreName _output_get)) (Utilities|Text|ToText(Name) InName)))
    (:then_1
      (Progress|SetPercent (Variables|/Game/Space/Ores/Widgets/WG_OreHealth.WG_OreHealth_C|GetProgressBar (Variables|/Game/Space/Ores/Widgets/WG_Meteor.WG_Meteor_C|GetWG_DamageProgress _output_get)) 1.0)
      (Class|ProgressBar|SetFillColorandOpacity (Variables|/Game/Space/Ores/Widgets/WG_OreHealth.WG_OreHealth_C|GetProgressBar (Variables|/Game/Space/Ores/Widgets/WG_Meteor.WG_Meteor_C|GetWG_DamageProgress _output_get)) Color)
      (Class|ProgressBar|SetFillColorandOpacity (Variables|/Game/Space/Ores/Widgets/WG_OreHealth.WG_OreHealth_C|GetProgressBar (Variables|/Game/Space/Ores/Widgets/WG_Meteor.WG_Meteor_C|GetWG_HpProgress _output_get)) Color))))

(fn UpdateWidget
  (bind _meteor_widget (Variables|Default|GetMeteor%20Widget)
    (:then
      (Progress|SetPercent (Variables|/Game/Space/Ores/Widgets/WG_OreHealth.WG_OreHealth_C|GetProgressBar (Variables|/Game/Space/Ores/Widgets/WG_Meteor.WG_Meteor_C|GetWG_HpProgress _meteor_widget)) (Pure|GetPrecentage))
      (Progress|SetPercent (Variables|/Game/Space/Ores/Widgets/WG_OreHealth.WG_OreHealth_C|GetProgressBar (Variables|/Game/Space/Ores/Widgets/WG_Meteor.WG_Meteor_C|GetWG_DamageProgress _meteor_widget)) (Pure|GetLittlePrecentage)))
    (:else)))

(fn GetPrecentage
  (return (/ (Math|Conversions|ToFloat(Integer) (Variables|HP|GetHp)) (Math|Conversions|ToFloat(Integer) (Variables|HP|GetMaxHp)))))

(fn GetLittlePrecentage
  (bind _hpper_unit (Variables|HP|GetHPPer%20Unit))
  (bind _hpper_unit_2 (Variables|HP|GetHPPer%20Unit))
  (bind _damagetaken (Variables|HP|GetDamageTaken))
  (bind _returnvalue (Math|Conversions|ToFloat(Integer) _hpper_unit))
  (bind _returnvalue_2 (- _hpper_unit_2 _damagetaken))
  (bind _returnvalue_3 (Math|Conversions|ToFloat(Integer) _returnvalue_2))
  (bind _returnvalue_4 (/ _returnvalue_3 _returnvalue))
  (if (<= _returnvalue_4 0.0)
    (return 1.0)
    (else
      (return _returnvalue_4))))