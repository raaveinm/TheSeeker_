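; BP_FloorBoard is a ship tile actor that shows, hides and re-materials its TileMesh according to tile state.
; Beyond hides the mesh; Wall, Floor and Doorway show it with BasicShapeMaterial, while Object and Trigger show it with no material specified.
; Cursor events set a scalar material parameter for hover, though the mesh's end-hover sets 1 rather than 0.
; Construction and BeginPlay both create dynamic material instances; highlighting and textures remain TODO.
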(event OnBeginCursorOver(TileMesh)
  (params (TouchedComponent :type Primitive%20Component%20Object%20Reference))
  ;[0.15 0.15 0.15 0.5] Cursor hover
  (Rendering|Material|SetScalarParameterValue 0 (Variables|Default|GetParameter%20Name) 1.0 :!class /Script/Engine.KismetMaterialLibrary))

(event OnEndCursorOver(TileMesh)
  (params (TouchedComponent :type Primitive%20Component%20Object%20Reference))
  ;[0.15 0.15 0.15 0.5] Cursor hover
  (Rendering|Material|SetScalarParameterValue 0 (Variables|Default|GetParameter%20Name) 1.0 :!class /Script/Engine.KismetMaterialLibrary))

(event OnComponentPhysicsStateChanged(TileMesh)
  (params (ChangedComponent :type Primitive%20Component%20Object%20Reference) (StateChange :type EComponentPhysicsStateChange%20Enum :default "Created")))

(event EventBeginPlay
  (Rendering|Material|CreateDynamicMaterialInstance (Variables|Default|GetTileMesh) 0 (Variables|Default|GetSource%20Material) "None" :!class /Script/Engine.PrimitiveComponent))

(event MouseInput|EventActorBeginCursorOver
  ;[0.15 0.15 0.15 0.5] Cursor hover
  (Rendering|Material|SetScalarParameterValue 0 (Variables|Default|GetParameter%20Name) 1.0 :!class /Script/Engine.KismetMaterialLibrary))

(event MouseInput|EventActorEndCursorOver
  ;[0.15 0.15 0.15 0.5] Cursor hover
  (Rendering|Material|SetScalarParameterValue 0 (Variables|Default|GetParameter%20Name) 0.0 :!class /Script/Engine.KismetMaterialLibrary))

(event EventOnTileStateChanged
  (params (NewState :type ETileState%20Enum :default "Beyond"))
  (bind _tilemesh (Variables|Default|GetTileMesh))
  (bind _tilemesh_2 (Variables|Default|GetTileMesh))
  ;[0.15 0.15 0.15 0.5] Tile changes
  (switch Utilities|FlowControl|Switch|SwitchonETileState NewState
    (:Beyond
      (Development|SetHiddeninGame _tilemesh true false))
    (:Wall
      (Development|SetHiddeninGame _tilemesh false false :!label _label)
      ;[0.15 0.15 0.15 0.5] #TODO - HIGHLIGHT MATERIAL & INTERACTION
      (Rendering|Material|SetMaterial _tilemesh_2 0 "/Engine/BasicShapes/BasicShapeMaterial.BasicShapeMaterial"))
    (:Floor
      (goto _label))
    (:Object
      (Development|SetHiddeninGame _tilemesh false false :!label _label_2)
      (Rendering|Material|SetMaterial _tilemesh_2 0 0))
    (:Trigger
      (goto _label_2))
    (:Doorway
      (goto _label))))

(fn ConstructionScript
  ;[0.15 0.15 0.15 0.5] #TODO - implement textures
  (Rendering|Material|CreateDynamicMaterialInstance (Variables|Default|GetTileMesh) 0 (Variables|Default|GetSource%20Material) "None" :!class /Script/Engine.PrimitiveComponent))